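; BP_Enemy is a monster that roams, chases the player and reloads FirstPersonMap when the first-person character enters its KillBox.
; PawnSensing sightings set a short-lived seen flag that drives a clamped detection score on Tick, switching aggression at a threshold.
; Aggressive, it chases at chase speed while the player is seen; otherwise it roams random navmesh points and periodically teleports between BP_TeleportPoint actors.
; A timed heartbeat sound plays when the player is near.
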(event OnSeePawn(PawnSensing)
  (params (Pawn :type Pawn%20Object%20Reference))
  ;[0 0 0 0.5] Detect if player is in enemy FOV
  (Variables|PlayerRelatedVariables|SetPlayerPawn Pawn)
  (Variables|EnemyBehavouirVariables|SetHasSeenPlayer true)
  (Utilities|FlowControl|Sequence
    (:then_0
      (Development|PrintString (Utilities|String|ToString(Boolean) (Variables|EnemyBehavouirVariables|GetHasSeenPlayer))))
    (:then_1
      (Utilities|FlowControl|RetriggerableDelay 0.6)
      (Variables|EnemyBehavouirVariables|SetHasSeenPlayer false))))

(event OnComponentBeginOverlap(KillBox)
  (params (OverlappedComponent :type Primitive%20Component%20Object%20Reference) (OtherActor :type Actor%20Object%20Reference) (OtherComp :type Primitive%20Component%20Object%20Reference) (OtherBodyIndex :type Integer) (bFromSweep :type Boolean) (SweepResult :type Hit%20Result%20Structure%20%28by%20ref%29))
  ;[0 0 0 0.5] Hit detection
  (Utilities|Casting|CastToBP_FirstPersonCharacter OtherActor)
  (Game|OpenLevel(byName) "FirstPersonMap"))

(event Custom|Follow%20Player
  ;[0 0 0 0.5] Chase Player
  (if (Variables|EnemyBehavouirVariables|GetHasSeenPlayer)
    (CallFunction|SetEnemySpeed (Variables|EnemySpeedVariables|GetChaseSpeed))
    (AI|AIMoveTo self "0, 0, 0" (Game|Player|GetPlayerPawn 0) 5.0 false)))

(event Custom|Roam
  ;[0 0 0 0.5] Roaming
  (Utilities|FlowControl|Delay 5.0)
  (CallFunction|SetEnemySpeed (Variables|EnemySpeedVariables|GetRoamSpeed))
  (bind _randomlocation (Class|NavigationSystemV1|GetRandomLocationinNavigableRadius (Transformation|GetActorLocation) 5e+03 0 0))
  (AI|AIMoveTo self _randomlocation 0 5.0 false))

(event EventBeginPlay
  (Variables|PlayerRelatedVariables|SetPlayerPawn (Game|GetPlayerCharacter 0))
  (bind _outactors (Actor|GetAllActorsOfClass "/Game/EnemyAI/BP_TeleportPoint.BP_TeleportPoint_C"))
  (Variables|EnemyTeleportBehavouir|SetTeleport%20Points _outactors))

(event EventTick
  (params (DeltaSeconds :type Float%20%28single-precision%29))
  (Variables|Default|SetDeltaTime DeltaSeconds)
  (Utilities|FlowControl|Sequence
    (:then_0
      ;[0 0 0 0.5] Detection
      (if (Variables|EnemyBehavouirVariables|GetHasSeenPlayer)
        (Utilities|FlowControl|Delay 0.2)
        (Variables|DetectionVariables|SetDetectionPercent (Math|Float|Clamp(Float) (+ (Variables|DetectionVariables|GetDetectionIncrement) (Variables|DetectionVariables|GetDetectionPercent)) 0.0 1e+02))
        (Development|PrintString (Utilities|String|ToString(Float) (Variables|DetectionVariables|GetDetectionPercent)))
        (else
          (Utilities|FlowControl|Delay 5.0)
          (Variables|DetectionVariables|SetDetectionPercent (Math|Float|Clamp(Float) (- (Variables|DetectionVariables|GetDetectionDecrement) (Variables|DetectionVariables|GetDetectionPercent)) 0.0 1e+02))
          (Development|PrintString (Utilities|String|ToString(Float) (Variables|DetectionVariables|GetDetectionPercent))))))
    (:then_1
      (if (>= (Variables|DetectionVariables|GetDetectionPercent) 5e+01)
        (Variables|EnemyBehavouirVariables|SetIsAggressive true)
        (else
          (Variables|EnemyBehavouirVariables|SetIsAggressive false))))
    (:then_2
      (if (Variables|EnemyBehavouirVariables|GetIsAggressive)
        (CallFunction|FollowPlayer)
        (else
          (CallFunction|Roam))))
    (:then_3
      ;[0 0 0 0.5] Teleport To Points
      (if (not (Variables|EnemyBehavouirVariables|GetIsAggressive))
        (Utilities|FlowControl|Delay (Variables|EnemyTeleportBehavouir|GetTeleportInterval))
        (Transformation|SetActorLocation (Transformation|GetActorLocation (Utilities|Array|Get(acopy) (Variables|EnemyTeleportBehavouir|GetTeleport%20Points) (Math|Random|RandomInteger (Utilities|Array|Length (Variables|EnemyTeleportBehavouir|GetTeleport%20Points))))) false false)
        (Development|PrintString "TELEPORTED")))
    (:then_5
      (Utilities|IsValid (Variables|PlayerRelatedVariables|GetPlayerPawn)
        (:Is%20Valid
          ;[0 0 0 0.5] SFX
          (if (< (Math|Vector|Distance(Vector) (Transformation|GetActorLocation) (Transformation|GetActorLocation (Variables|PlayerRelatedVariables|GetPlayerPawn))) 1.5e+03)
            (if (>= (Variables|SFXVariables|GetMonsterSFXTimer) (Variables|SFXVariables|GetMonsterSFXInterval))
              (Variables|SFXVariables|SetMonsterSFXTimer 0.0)
              (Audio|PlaySound2D (Variables|SFXVariables|GetHeartBeatSFX) 1.0 1.0 0.0 0 0)
              (else
                (Variables|SFXVariables|SetMonsterSFXTimer (+ (Variables|SFXVariables|GetMonsterSFXTimer) (Variables|Default|GetDeltaTime)))))))))))

(fn ConstructionScript)

(fn SetEnemySpeed
  (params (NewSpeed :type Float%20%28double-precision%29))
  (Variables|/Script/Engine.CharacterMovementComponent|SetMaxWalkSpeed (Variables|Character|GetCharacterMovement) NewSpeed))