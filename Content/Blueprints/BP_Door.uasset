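; BP_Door is an automatic sliding double door that opens when something enters its Box trigger and closes when it leaves.
; Overlap events play or reverse the OpenCloseDoor timeline, whose DoorTrack lerps Door1 and Door2 apart in opposite directions along local Y.
; Each overlap also swaps an emissive material on the Frame and plays a metal door sound, with no filter on the overlapping actor.
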(event OnComponentEndOverlap(Box)
  (params (OverlappedComponent :type Primitive%20Component%20Object%20Reference) (OtherActor :type Actor%20Object%20Reference) (OtherComp :type Primitive%20Component%20Object%20Reference) (OtherBodyIndex :type Integer))
  (Rendering|Material|SetMaterial (Variables|Default|GetFrame) 1 "/Game/Models/models_props/MehanicalDoorEmission1.MehanicalDoorEmission1")
  (Audio|Components|Audio|Play (Variables|Default|GetMetalDoorSound) 0.0)
  (bind _door_track (Timeline|Open/Close%20Door Reverse)
    (:Update
      (Transformation|SetRelativeLocation (Variables|Default|GetDoor1) (Math|Vector|MakeVector 0.0 (Math|Float|Lerp 0.0 1.4e+02 _door_track) 0.0) false false)
      (Transformation|SetRelativeLocation (Variables|Default|GetDoor2) (Math|Vector|MakeVector 0.0 (Math|Float|Lerp 0.0 -1.4e+02 _door_track) 0.0) false false))))

(event OnComponentBeginOverlap(Box)
  (params (OverlappedComponent :type Primitive%20Component%20Object%20Reference) (OtherActor :type Actor%20Object%20Reference) (OtherComp :type Primitive%20Component%20Object%20Reference) (OtherBodyIndex :type Integer) (bFromSweep :type Boolean) (SweepResult :type Hit%20Result%20Structure%20%28by%20ref%29))
  (Rendering|Material|SetMaterial (Variables|Default|GetFrame) 1 "/Game/Models/models_props/MehanicalDoorEmission.MehanicalDoorEmission")
  (Audio|Components|Audio|Play (Variables|Default|GetMetalDoorSound) 0.0)
  (bind _door_track (Timeline|Open/Close%20Door Play)
    (:Update
      (Transformation|SetRelativeLocation (Variables|Default|GetDoor1) (Math|Vector|MakeVector 0.0 (Math|Float|Lerp 0.0 1.4e+02 _door_track) 0.0) false false)
      (Transformation|SetRelativeLocation (Variables|Default|GetDoor2) (Math|Vector|MakeVector 0.0 (Math|Float|Lerp 0.0 -1.4e+02 _door_track) 0.0) false false))))

(fn ConstructionScript)