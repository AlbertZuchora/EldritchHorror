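; Double door actor that the player opens and closes with E while inside its sphere trigger, optionally requiring a key card.
; Overlap toggles input, and a dot product against the door's forward vector sets the swing direction on opening.
; Two timelines rotate the leaves in opposite directions.
; If flagged, the left timeline's update triggers a one-time outro video widget, pauses the game and loads the main menu after a delay.
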(event OnComponentBeginOverlap(Sphere)
  (params (OverlappedComponent :type Primitive%20Component%20Object%20Reference) (OtherActor :type Actor%20Object%20Reference) (OtherComp :type Primitive%20Component%20Object%20Reference) (OtherBodyIndex :type Integer) (bFromSweep :type Boolean) (SweepResult :type Hit%20Result%20Structure%20%28by%20ref%29))
  (Utilities|Casting|CastToBP_FirstPersonCharacter OtherActor)
  (Input|EnableInput (Game|GetPlayerController 0)))

(event OnComponentEndOverlap(Sphere)
  (params (OverlappedComponent :type Primitive%20Component%20Object%20Reference) (OtherActor :type Actor%20Object%20Reference) (OtherComp :type Primitive%20Component%20Object%20Reference) (OtherBodyIndex :type Integer))
  (Utilities|Casting|CastToBP_FirstPersonCharacter OtherActor)
  (Input|DisableInput (Game|GetPlayerController 0)))

(event Collision|EventActorBeginOverlap
  (params (OtherActor :type Actor%20Object%20Reference)))

(event EventTick
  (params (DeltaSeconds :type Float%20%28single-precision%29)))

(event Input|KeyboardEvents|E
  (params (Key :type Key%20Structure :default "None"))
  (:Pressed
    (Audio|Components|Audio|Play (Variables|Default|GetDoorSound) 0.01)
    (bind _asbp_first_person_character (Utilities|Casting|CastToBP_FirstPersonCharacter (Game|GetPlayerCharacter 0)))
    ;[0.15 0.1344 0.0464 0.5] Check if door needs key card and if player has key card.
    (if (Variables|Default|GetRequiresKeyCard)
      (if (Variables|/Game/FirstPerson/Blueprints/BP_FirstPersonCharacter.BP_FirstPersonCharacter_C|GetPlayerHasKeyCard _asbp_first_person_character)
        (if (Variables|Default|GetIsOpen) :!label _label
          (Utilities|FlowControl|Sequence
            (:then_0
              (bind _rightdoortrack (Timeline|RightDoorAnimation Reverse)
                (:Update
                  (Transformation|SetRelativeRotation (Variables|Default|GetRightDoor) (Math|Rotator|MakeRotator 0.0 0.0 (Math|Float|Lerp 0.0 (* (Variables|Default|GetOpenDirection) -9e+01) _rightdoortrack)) false false))))
            (:then_1
              (bind _leftdoortrack (Timeline|LeftDoorAnimation Reverse)
                (:Update
                  (Transformation|SetRelativeRotation (Variables|Default|GetLeftDoor) (Math|Rotator|MakeRotator 0.0 0.0 (Math|Float|Lerp 0.0 (* (Variables|Default|GetOpenDirection) 9e+01) _leftdoortrack)) false false)
                  (if (Variables|Default|GetPlayCutscene)
                    (if (not (Variables|Default|GetHasPlayedCutscene))
                      (Variables|Default|SetHasPlayedCutscene true)
                      (bind _returnvalue (UserInterface|CreateWidget "/Game/UI/WBP_Cutscene.WBP_Cutscene_C" 0 "/Game/Movies/MediaPlayer.MediaPlayer" "/Game/Movies/OutroVideo.OutroVideo"))
                      (UserInterface|Viewport|AddtoViewport _returnvalue 0)
                      (Game|SetGamePaused true)
                      (Utilities|FlowControl|Delay 0.1)
                      (Game|OpenLevel(byName) "MainMenu2"))))))
            (:then_2
              (Variables|Default|SetIsOpen false)))
          (else
            (if (> (Math|Vector|DotProduct (Math|Vector|Normalize (- (Transformation|GetActorLocation (Game|GetPlayerCharacter 0)) (Transformation|GetActorLocation))) (Math|Vector|GetForwardVector (Variables|Components|GetDefaultSceneRoot))) 0.0)
              (Variables|Default|SetOpenDirection 1.0)
              (else
                (Variables|Default|SetOpenDirection -1.0)))
            (Utilities|FlowControl|Sequence
              (:then_0
                (Timeline|RightDoorAnimation PlayFromStart))
              (:then_1
                (Timeline|LeftDoorAnimation PlayFromStart))
              (:then_2
                (Variables|Default|SetIsOpen true))))))
      (else
        (goto _label)))))

(fn ConstructionScript)