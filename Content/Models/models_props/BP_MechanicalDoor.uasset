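; BP_MechanicalDoor is a two-panel mechanical door that slides open and closed when its OpenDoor event is called.
; A FlipFlop alternates between playing OpenDoorTimeline from the start and reversing it, with its two tracks setting each panel's relative Y position and zeroing X and Z.
; BeginPlay stores both panels' start locations, but the movement ignores them.
; A delayed auto-close branch is left disconnected and never runs.
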(event Custom|OpenDoor
  (Utilities|FlowControl|FlipFlop
    (:A
      (bind (_direction _door_l _door_r) (Timeline|Open%20Door%20Timeline PlayFromStart)
        (:Update
          (Utilities|FlowControl|Sequence
            (:then_0
              (Transformation|SetRelativeLocation (Variables|Default|GetDoor_L) (Math|Vector|MakeVector 0.0 _door_l 0.0) false false))
            (:then_1
              (Transformation|SetRelativeLocation (Variables|Default|GetDoor_R) (Math|Vector|MakeVector 0.0 _door_r 0.0) false false))))))
    (:B
      (Timeline|Open%20Door%20Timeline Reverse))))

(event EventBeginPlay
  (Utilities|FlowControl|Sequence
    (:then_0
      (Variables|Default|SetLeftDoor_startLocation (Variables|/Script/Engine.SceneComponent|GetRelativeLocation (Variables|Default|GetDoor_L))))
    (:then_1
      (Variables|Default|SetRightDoor_startLocation (Variables|/Script/Engine.SceneComponent|GetRelativeLocation (Variables|Default|GetDoor_R))))))

(fn ConstructionScript)