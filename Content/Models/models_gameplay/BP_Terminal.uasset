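; BP_Terminal is an interactable terminal that opens a readable screen when the player uses it.
; Its Interact function calls TerminalInteract and returns the terminal's static mesh to the caller.
; TerminalInteract creates a WBP_InteractText widget showing the terminal's texture, plays a click sound, then pauses the game and switches to UI-only input with the mouse cursor shown.
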(event Custom|Terminal%20Interact
  (bind _returnvalue (Game|GetPlayerController 0))
  (bind _returnvalue_2 (UserInterface|CreateWidget "/Game/UI/WBP_InteractText.WBP_InteractText_C" (Game|GetPlayerController 0)))
  (bind _output_get (Variables|Default|SetTerminalWidget _returnvalue_2))
  (Default|SetTerminalTexture _output_get (Variables|Default|GetTerminalTexture))
  (Audio|Components|Audio|Play (Variables|Default|GetMouseClick) 0.0)
  (UserInterface|Viewport|AddtoViewport (Variables|Default|GetTerminalWidget) 0)
  (Game|SetGamePaused true)
  (Input|SetInputModeUIOnly _returnvalue (Variables|Default|GetTerminalWidget) "DoNotLock" false)
  (Variables|/Script/Engine.PlayerController|SetbShowMouseCursor _returnvalue true))

(fn ConstructionScript)

(fn Interact
  (CallFunction|TerminalInteract)
  (return (Variables|/Script/Engine.StaticMeshComponent|GetStaticMesh (Variables|Default|GetTerminal))))